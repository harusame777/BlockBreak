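; BP_Block is a breakable block that loses one point of strength each time a BP_Ball hits it.
; At zero strength it spawns an explosion emitter at its location and destroys itself; otherwise it refreshes its color.
; UpdateBlockColor swaps the mesh material to yellow, red or green by remaining strength, and the construction script also calls it so the starting color matches BlockStrength.
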(event EventBeginPlay)

(event Collision|EventActorBeginOverlap
  (params (OtherActor :type Actor%20Object%20Reference)))

(event EventTick
  (params (DeltaSeconds :type Float%20%28single-precision%29)))

(event Collision|EventHit
  (params (MyComp :type Primitive%20Component%20Object%20Reference) (Other :type Actor%20Object%20Reference) (OtherComp :type Primitive%20Component%20Object%20Reference) (bSelfMoved :type Boolean) (HitLocation :type Vector :default "0, 0, 0") (HitNormal :type Vector :default "0, 0, 0") (NormalImpulse :type Vector :default "0, 0, 0") (Hit :type Hit%20Result%20Structure%20%28by%20ref%29))
  (Utilities|Casting|CastToBP_Ball Other)
  (bind _result (Math|Integer|DecrementInt (Variables|Default|GetBlockStrength))
    (:%20%20
      (if (== _result 0)
        (Effects|SpawnEmitteratLocation "/Game/StarterContent/Particles/P_Explosion.P_Explosion" (Transformation|GetActorLocation))
        (Actor|DestroyActor)
        (else
          (CallFunction|UpdateBlockColor))))))

(fn ConstructionScript
  (CallFunction|UpdateBlockColor))

(fn UpdateBlockColor
  (bind _ksm_block (Variables|Default|GetKSM_Block))
  (switch int (Variables|Default|GetBlockStrength)
    (:1
      (Rendering|Material|SetMaterial _ksm_block 0 "/Game/Materials/INST_Yellow.INST_Yellow"))
    (:2
      (Rendering|Material|SetMaterial _ksm_block 0 "/Game/Materials/INST_Red.INST_Red"))
    (:3
      (Rendering|Material|SetMaterial _ksm_block 0 "/Game/Materials/INST_Green.INST_Green"))))